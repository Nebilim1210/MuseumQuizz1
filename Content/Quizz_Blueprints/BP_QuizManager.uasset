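; Quiz manager Blueprint that runs a session of randomly picked questions from DT_QuestionList.
; The construction script builds the session by shuffling the table's row names and taking TotalQuestions rows.
; BeginPlay creates WBP_QuestionWidget, displays the current question and binds OnAnswerSelected to CheckAnswer, which prints whether the pick matches the first correct answer.
; LoadNextQuestion increments the index but is not called in this Blueprint.
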(event Custom|AskQuestionEvent
  (bind _questionwidget (Variables|Default|GetQuestionWidget))
  (bind _output (CallFunction|GetCurrentQuestion))
  (Default|DisplayQuestion _questionwidget _output) ; Set the question widget so it registers the question to display
  (EventDispatchers|BindEventtoOnAnswerSelected _questionwidget (delegate Custom|CheckAnswerEvent)) ; Asks the QuizManager to listen for which answer will be selected !
  (UserInterface|Viewport|AddtoViewport (Variables|Default|GetQuestionWidget) 0))

(event Custom|CheckAnswerEvent
  (params (SelectedAnswer :type Text))
  (CallFunction|CheckAnswer SelectedAnswer))

(event EventBeginPlay
  (bind _returnvalue (UserInterface|CreateWidget "/Game/Quizz_UI/WBP_QuestionWidget.WBP_QuestionWidget_C"))
  (Variables|Default|SetQuestionWidget _returnvalue)
  (CallFunction|AskQuestionEvent))

(event Collision|EventActorBeginOverlap
  (params (OtherActor :type Actor%20Object%20Reference)))

(event EventTick
  (params (DeltaSeconds :type Float%20%28single-precision%29)))

(fn ConstructionScript
  (bind _questionsreturned (CallFunction|BuildQuestionPanel))
  (bind _output_get (Variables|Default|SetSessionsQuestionsPanel _questionsreturned))
  (Variables|Default|SetCurrentQuestionIndex 0)
  (Variables|Default|SetTotalQuestions (Utilities|Array|Length _output_get)))

(fn LoadNextQuestion
  ;[1 1 1] Vérifie si nous sommes toujours dans les limites du nombre de questions, et si c'est le cas, passe à la question suivante
  (if (Utilities|Array|IsValidIndex (Variables|Default|GetSessionsQuestionsPanel) (Variables|Default|GetCurrentQuestionIndex))
    (bind _result (Math|Integer|IncrementInt (Variables|Default|GetCurrentQuestionIndex))
      (:%20%20
        (Variables|Default|SetCurrentQuestionIndex _result)))))

(fn GetCurrentQuestion
  ;[1 1 1] On récupère la question et les réponses de la question actuellement posée
  (return (Utilities|Array|Get(acopy) (Variables|Default|GetSessionsQuestionsPanel) (Variables|Default|GetCurrentQuestionIndex))))

(fn BuildQuestionPanel
  (bind _outrownames (DataTable|GetDataTableRowNames "/Game/Quizz_Blueprints/DT_QuestionList.DT_QuestionList"))
  (Variables|Default|SetAllQuestionsIDs _outrownames)
  (Utilities|Array|Shuffle (Variables|Default|GetAllQuestionsIDs)) ; We shuffle the array in order to get random questions when picking the top
  (for _index (range 0 (- (Variables|Default|GetTotalQuestions) 1))
    ;[1 1 1] At each step of the loop : We take a random question name, add its data to the returned array of questions, and remove it from our panel at the end
    (bind _returnvalue (Utilities|GetDataTableRow "/Game/Quizz_Blueprints/DT_QuestionList.DT_QuestionList" (Utilities|Array|Get(acopy) (Variables|Default|GetAllQuestionsIDs) _index))
      (:then
        (Utilities|Array|Add (LocalVariables|GetReturnedQuestions) _returnvalue))))
  (return (LocalVariables|GetReturnedQuestions)))

(fn CheckAnswer
  (params (SelectedAnswer :type Text))
  (bind _output (CallFunction|GetCurrentQuestion))
  (if (Utilities|Enum|Equal(Enum) (Utilities|Array|Get(acopy) (.AnswerOptions (Utilities|Struct|BreakST_QuestionData _output)) (Utilities|Array|Get(acopy) (.CorrectAnswers (Utilities|Struct|BreakST_QuestionData _output)))) SelectedAnswer)
    (Development|PrintString "Bonne réponse !")
    (else
      (Development|PrintString "Mauvaise réponse"))))