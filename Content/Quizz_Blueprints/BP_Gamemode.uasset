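; Game mode Blueprint for a quiz game that creates and holds the quiz manager.
; The StartNewQuizz event spawns a BP_QuizManager actor and stores it as GameQuizManager, which a getter exposes.
; PrintQuestion asks that manager for the current question and prints its text.
; A FIXME on the spawn step notes that spawning must happen in the game mode.
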(event Custom|StartNewQuizz
  (bind _returnvalue (Game|SpawnActorfromClass "/Game/Quizz_Blueprints/BP_QuizManager.BP_QuizManager_C" (Variables|Default|GetSpawn%20Transform) "Undefined" "MultiplyWithRoot" 0 0)) ; FIXME : Doit Spawner dans le Gamemode
  (Variables|Default|SetGameQuizManager _returnvalue))

(fn ConstructionScript)

(fn GetGameQuizManager
  (return (Variables|Default|GetGameQuizManager)))

(fn PrintQuestion
  (bind _output (Default|GetCurrentQuestion (Variables|Default|GetGameQuizManager)))
  (Development|PrintText (.QuestionText (Utilities|Struct|BreakST_QuestionData _output))))